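; Battery manager Blueprint that scatters a configurable number of actors, presumably batteries, across the level when play begins.
; BeginPlay runs a counter loop up to NbBatteries, spawning one actor per pass at a random X/Y position within a fixed square centered on the world origin, with random yaw.
; Tick, overlap and construction logic are empty, so all work happens once at startup.
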(event `self.ReceiveBeginPlay`
  (set `self.iBatteries` 0)
  (while (< (`self.iBatteries`) (`self.nbBatteries`))
    (`|SpawnActorFromClass` "/Game/Assets/battery_BP.battery_BP_C" (`KismetMathLibrary.MakeTransform` (`KismetMathLibrary.MakeVector` (`KismetMathLibrary.RandomFloatInRange` -1820.0 1820.0) (`KismetMathLibrary.RandomFloatInRange` -1820.0 1820.0)) (`KismetMathLibrary.MakeRotator` 0.0 0.0 (`KismetMathLibrary.RandomFloatInRange` -180.0 180.0))) "Undefined" "MultiplyWithRoot" null null)
    (bind _result (`/Engine/EditorBlueprintResources/StandardMacros.IncrementInt` (`self.iBatteries`))
      (:`  `
        (set `self.iBatteries` _result)))))

(fn `UserConstructionScript`)
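; Battery-powered door actor that rises open when the player overlaps it with enough batteries, deducting the cost and switching on its spotlight.
; BeginPlay caches the first-person character, stores and zeroes the light intensity, and computes the target height from OpenZ.
; Tick raises the Porte component at DoorSpeed until it reaches that height.
; Once the door is past that height, further player overlaps toggle the spotlight through a FlipFlop.
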(event `self.ReceiveBeginPlay`
  (bind _spotlight (`self.SpotLight`))
  (bind (_returnvalue_x _returnvalue_y _returnvalue_z) (`KismetMathLibrary.BreakVector` (`SceneComponent.K2_GetComponentLocation` (`self.Porte`))))
  (set `self.LightIntensity` (`LightComponentBase.Intensity` _spotlight))
  (`LightComponent.SetIntensity` _spotlight 0.0)
  (bind _asbp_first_person_character (cast `/Game/FirstPerson/Blueprints/BP_FirstPersonCharacter` (`GameplayStatics.GetPlayerCharacter` 0)))
  (set `self.Player` _asbp_first_person_character)
  (set `self.doorEndPos` (+ (`self.OpenZ`) _returnvalue_z)))

(event `self.ReceiveActorBeginOverlap`
  (params (OtherActor :type "Actor Object Reference"))
  (bind _player (`self.Player`))
  (bind _batteriesneeded (`self.batteriesNeeded`))
  (bind (_returnvalue_x _returnvalue_y _returnvalue_z) (`KismetMathLibrary.BreakVector` (`SceneComponent.K2_GetComponentLocation` (`self.Porte`))))
  (bind _batterynb (`/Game/FirstPerson/Blueprints/BP_FirstPersonCharacter.batteryNb` _player))
  (if (`self.ActorHasTag` OtherActor "Player")
    (if (> _returnvalue_z (`self.doorEndPos`))
      (bind _isa (`/Engine/EditorBlueprintResources/StandardMacros.FlipFlop`)
        (:`A`
          _)
        (:`B`
          _))
      (`LightComponent.SetIntensity` (`self.SpotLight`) (`KismetMathLibrary.SelectFloat` (`self.LightIntensity`) 0.0 _isa))
      (elif (>= _batterynb _batteriesneeded)
        (set `/Game/FirstPerson/Blueprints/BP_FirstPersonCharacter.batteryNb` (- _batterynb _batteriesneeded) _player)
        (`LightComponent.SetIntensity` (`self.SpotLight`) (`self.LightIntensity`))
        (set `self.doorOpening` true)))))

(event `self.ReceiveTick`
  (params (DeltaSeconds :type "Float (single-precision)"))
  (bind _porte (`self.Porte`))
  (bind (_returnvalue_x _returnvalue_y _returnvalue_z) (`KismetMathLibrary.BreakVector` (`SceneComponent.K2_GetComponentLocation` _porte)))
  (bind (_returnvalue_x_2 _returnvalue_y_2 _returnvalue_z_2) (`KismetMathLibrary.BreakVector` (`SceneComponent.K2_GetComponentLocation` _porte)))
  (if (`self.doorOpening`)
    (`SceneComponent.K2_SetWorldLocation` _porte (`KismetMathLibrary.MakeVector` _returnvalue_x_2 _returnvalue_y_2 (+ _returnvalue_z_2 (* (`self.doorSpeed`) DeltaSeconds))) false false)
    (set `self.doorOpening` (< _returnvalue_z (`self.doorEndPos`)))))

(fn `UserConstructionScript`)